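; Base robot Blueprint, named as an old version, that runs a task held in CurrentTask.
; ExecuteNewTask switches on the task type to fire a Say Hello or Go To event.
; Both events use delays to simulate work and set TaskState to Finished, but only Say Hello marks it Running first and prints the task's message.
; Go To only prints and waits, with no actual movement.
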(event `self.ReceiveTick`
  (params (DeltaSeconds :type "Float (single-precision)")))

(event `SayHelloEvent`
  (bind (_currenttask_tasktype _currenttask_hellomessage) (break `/Game/Data/S_RobotTask` (`self.CurrentTask`)))
  (`KismetSystemLibrary.PrintString` "Receive Message:")
  (set `self.TaskState` "Running")
  (`KismetSystemLibrary.Delay` 5.0)
  (`KismetSystemLibrary.PrintString` _currenttask_hellomessage)
  (set `self.TaskState` "Finished"))

(event `MoveToEvent`
  (`KismetSystemLibrary.PrintString` "Moving")
  (`KismetSystemLibrary.Delay` 2.0)
  (set `self.TaskState` "Finished"))

(fn `ExecuteNewTask`
  (bind _currenttask_tasktype (break `/Game/Data/S_RobotTask` (`self.CurrentTask`)))
  (switch `/Game/Data/E_TaskType` _currenttask_tasktype
    (:`NewEnumerator1`
      (`self.SayHelloEvent`))
    (:`NewEnumerator2`
      (`self.MoveToEvent`))))

(fn `UserConstructionScript`)