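; BP_RobotBaseController is a base AI controller for robots that starts the BT_Robot behavior tree on BeginPlay.
; HandleTaskRequest stores an incoming task as the active task and writes its type to a Blackboard enum that identifies which task data applies.
; GetActorByName linearly scans all world actors for BPI_NavigationTarget implementers and returns the one whose reported name matches, or nothing otherwise.
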(event `self.ReceiveBeginPlay`
  (`self.RunBehaviorTree` "/Game/Behavior/BT_Robot.BT_Robot"))

(fn `GetActorByName`
  (params (ActorIdentifier :type String))
  (returns (ActorFound :type "Actor Object Reference"))
  (bind _outactors (`GameplayStatics.GetAllActorsOfClass` "/Script/Engine.Actor"))
  (for _array_element _outactors
    (if (`KismetSystemLibrary.DoesImplementInterface` _array_element "/Game/Interfaces/BPI_NavigationTarget.BPI_NavigationTarget_C")
      (bind _uniqueidentifier (message `/Game/Interfaces/BPI_NavigationTarget.GetActorName` _array_element))
      (if (== _uniqueidentifier ActorIdentifier)
        (return _array_element))))
  ; Se nao achar, retorna vazio
  (return null))

(fn `HandleTaskRequest`
  (params (TaskEntry :type "/Game/Data/Task_HUB Structure"))
  ; Saves a copy of the new request. We can block new requests from the Actor if needed.
  (bind _output_get (set `self.ActiveTask` TaskEntry))
  ; Set the Blackboard type value so we can later identify which item in the struct will be used.
  (`BlackboardComponent.SetValueAsEnum` (`AIBlueprintHelperLibrary.GetBlackboard` null) (`self.TaskType_KeyName`) (break `/Game/Data/Task_HUB` _output_get)))

(fn `UserConstructionScript`)